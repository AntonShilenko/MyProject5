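; BP_Light is a Blueprint that blinks its point light a set number of times after play begins.
; After a one-second delay, a DoN node gated by Amount toggles the light's visibility twice, waiting Speed seconds after each toggle.
; The sequence loops back into the DoN until the count runs out, leaving the light in its starting visibility.
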(event EventBeginPlay
  (bind _speed (Variables|Default|GetSpeed))
  (Utilities|FlowControl|Delay 1.0)
  (Utilities|FlowControl|DoN (Variables|Default|GetAmount) :!label _label
    (:Exit
      (Rendering|ToggleVisibility (Variables|Default|GetPointLight) (Variables|Default|GetLight))
      (Utilities|FlowControl|Delay _speed)
      (Rendering|ToggleVisibility (Variables|Default|GetPointLight) (Variables|Default|GetLight))
      (Utilities|FlowControl|Delay _speed)
      (goto _label))))

(fn ConstructionScript)